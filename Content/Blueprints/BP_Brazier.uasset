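; BP_Brazier is a brazier actor that lights its Niagara effect when it visually lines up on screen with a linked sibling brazier, a perspective-alignment mechanic.
; Each Tick while the effect is inactive, it projects both CastPoints to screen space and compares them against X and Y accuracy thresholds.
; Construction feeds Stencil into the effect's User.Stencil parameter; BecomeNormal activates the effect and zeroes that parameter on this brazier only.
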(event EventBeginPlay
  (bind _returnvalue (Actor|GetActorOfClass "/Game/ThirdPerson/Blueprints/BP_ThirdPersonCharacter.BP_ThirdPersonCharacter_C"))
  (Variables|Default|SetPlayer _returnvalue))

(event EventTick
  (params (DeltaSeconds :type Float%20%28single-precision%29))
  (bind _returnvalue (Game|GetPlayerController 0))
  (bind _returnvalue_2 (Game|GetPlayerController 0))
  (bind _castpoint (Variables|Default|GetCastPoint))
  (bind _sibling (Variables|Default|GetSIbling))
  (bind _returnvalue_3 (Transformation|GetWorldLocation _castpoint))
  (bind _castpoint_2 (Variables|BP_Brazier_C|GetCastPoint _sibling))
  (bind _screenposition (Class|GameplayStatics|ProjectWorldtoScreen _returnvalue_2 _returnvalue_3 false))
  (bind _returnvalue_4 (Transformation|GetWorldLocation _castpoint_2))
  (bind _screenposition_2 (Class|GameplayStatics|ProjectWorldtoScreen _returnvalue _returnvalue_4 false))
  (if (and (Utilities|IsValid (Variables|Default|GetSIbling)) (not (Components|Activation|IsActive (Variables|Default|GetNiagaraSystem))))
    (if (and (< (Math|Float|Absolute(Float) (- (.x _screenposition) (.x _screenposition_2))) (Variables|Default|GetXAccuracy)) (< (Math|Float|Absolute(Float) (- (.y _screenposition) (.y _screenposition_2))) (Variables|Default|GetYAccuracy)))
      (CallFunction|BecomeNormal))))

(fn ConstructionScript
  (Niagara|SetNiagaraVariable(Float) (Variables|Default|GetNiagaraSystem) "User.Stencil" (Variables|Default|GetStencil)))

(fn BecomeNormal
  (Components|Activation|Activate (Variables|Default|GetNiagaraSystem) false)
  (Niagara|SetNiagaraVariable(Float) (Variables|Default|GetNiagaraSystem) "User.Stencil" 0.0))