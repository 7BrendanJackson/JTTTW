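; BP_GrassDetectionWaypoint is a waypoint actor with a trigger box that feeds a BP_GrassPathDetection path.
; On BeginPlay it finds the path through its root component's attach parent owner and registers itself with it.
; When a BP_RegrowthCharacter leaves the box, it tells the path to check progress.
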(event OnComponentEndOverlap(Box)
  (params (OverlappedComponent :type Primitive%20Component%20Object%20Reference) (OtherActor :type Actor%20Object%20Reference) (OtherComp :type Primitive%20Component%20Object%20Reference) (OtherBodyIndex :type Integer))
  (Utilities|Casting|CastToBP_RegrowthCharacter OtherActor)
  (Default|CheckProgress (Variables|Default|GetGrassDetectionPath)))

(event EventBeginPlay
  (bind _asbp_grass_path_detection (Utilities|Casting|CastToBP_GrassPathDetection (Components|GetOwner (Transformation|GetAttachParent (Variables|Default|GetDefaultSceneRoot)))))
  (bind _output_get (Variables|Default|SetGrassDetectionPath _asbp_grass_path_detection))
  (Default|RegisterWaypoint _output_get self))

(fn ConstructionScript)