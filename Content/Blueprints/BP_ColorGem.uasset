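; Interactable gem that restores or drains color on assigned static meshes and foliage, activating or deactivating linked I_Toggle actors as it switches.
; The construction script gathers the mesh components from assigned actors.
; Custom primitive data passes gem location, Size and completion level to their materials.
; A timeline, with play rate inversely proportional to Size, animates completion forward or backward on each interaction.
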(event EventInteract
  (if (Variables|Default|GetIsColorDrained?)
    (Variables|Default|SetIsColorDrained? (not (Variables|Default|GetIsColorDrained?)))
    (for _array_element (Variables|Default|GetEventTrigger)
      (if (Utilities|DoesObjectImplementInterface _array_element "/Game/Blueprints/Interfaces/I_Toggle.I_Toggle_C")
        (Class|IToggle|Activate(Message) _array_element)))
    (bind _level (Timeline|Timeline Play)
      (:Update
        (CallFunction|SetCompletionLevel _level)))
    (else
      (Variables|Default|SetIsColorDrained? (not (Variables|Default|GetIsColorDrained?)))
      (for _array_element_2 (Variables|Default|GetEventTrigger)
        (if (Utilities|DoesObjectImplementInterface _array_element_2 "/Game/Blueprints/Interfaces/I_Toggle.I_Toggle_C")
          (Class|IToggle|Deactivate(Message) _array_element_2)))
      (Timeline|Timeline Reverse))))

(event EventBeginPlay
  (Components|Timeline|SetPlayRate (Variables|Default|GetTimeline) (/ 5e+02 (Variables|Default|GetSize)))
  (CallFunction|SetCompletionLevel (select (Variables|Default|GetIsColorDrained?) 0.0 1.0))
  (CallFunction|SetDrainLocation))

(fn ConstructionScript
  (Utilities|Array|Clear (Variables|Default|GetDistancesToMesh))
  (Utilities|Array|Clear (Variables|Default|GetStaticMeshToDrain))
  (for _array_element (Variables|Default|GetActorToDrain)
    (bind _asstatic_mesh_actor (Utilities|Casting|CastToStaticMeshActor _array_element))
    (Utilities|Array|Add (Variables|Default|GetStaticMeshToDrain) (Variables|/Script/Engine.StaticMeshActor|GetStaticMeshComponent _asstatic_mesh_actor))
    (Utilities|Array|Add (Variables|Default|GetDistancesToMesh) (Math|Vector|Distance(Vector) (Transformation|GetWorldLocation (Variables|/Script/Engine.StaticMeshActor|GetStaticMeshComponent _asstatic_mesh_actor)) (Transformation|GetWorldLocation (Variables|Default|GetDiamond)))))
  (for _array_element_2 (Variables|Default|GetInstancedFoliageActor)
    (Utilities|Array|AppendArray (Variables|Default|GetInstancedMeshToDrain) (Actor|GetComponentsByClass _array_element_2 "/Script/Foliage.FoliageInstancedStaticMeshComponent")))
  (CallFunction|SetCompletionLevel (select (Variables|Default|GetIsColorDrained?) 0.0 1.0))
  (CallFunction|SetDrainLocation))

(fn SetCompletionLevel
  (params (Level :type Float%20%28double-precision%29))
  (for _array_element (Variables|Default|GetStaticMeshToDrain)
    ;[1 1 1] Completion
    (Rendering|Material|SetCustomPrimitiveDataFloat _array_element 3 Level))
  (for _array_element_2 (Variables|Default|GetInstancedMeshToDrain)
    (Rendering|Material|SetCustomPrimitiveDataFloat _array_element_2 3 Level)))

(fn SetDrainLocation
  (for _array_element (Variables|Default|GetStaticMeshToDrain)
    ;[1 1 1] Drain Location
    (Rendering|Material|SetCustomPrimitiveDataVector3 _array_element 4 (Transformation|GetActorLocation))
    ;[1 1 1] Size
    (Rendering|Material|SetCustomPrimitiveDataFloat _array_element 7 (Variables|Default|GetSize)))
  (for _array_element_2 (Variables|Default|GetInstancedMeshToDrain)
    ;[1 1 1] Drain Location
    (Rendering|Material|SetCustomPrimitiveDataVector3 _array_element_2 4 (Transformation|GetActorLocation))
    ;[1 1 1] Size
    (Rendering|Material|SetCustomPrimitiveDataFloat _array_element_2 7 (Variables|Default|GetSize))))