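; Foliage tree actor that grows its leaves when triggered and passes the event on to other actors.
; TriggerEvent plays the GrowLeaves timeline, writing its curve to the static mesh's custom primitive data to drive the growth.
; A timeline Trigger track activates leaf and butterfly particles, then messages SendTriggers entries implementing I_FoliageEvent, allowing chained reactions.
; The construction script scales the timeline play rate from LeavesGrowTime.
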(event EventBeginPlay)

(event Collision|EventActorBeginOverlap
  (params (OtherActor :type Actor%20Object%20Reference)))

(event EventTick
  (params (DeltaSeconds :type Float%20%28single-precision%29)))

(event EventTriggerEvent
  (bind _growleaves (Timeline|GrowLeaves Play)
    (:Update
      (Rendering|Material|SetCustomPrimitiveDataFloat (Variables|Debug|GetStaticMeshComponent) 0 _growleaves))
    (:Trigger
      (Components|Activation|Activate (Variables|Default|GetLeavesParticle) false)
      (Components|Activation|Activate (Variables|Default|GetButterflyParticle) false)
      (for _array_element (Variables|Default|GetSendTriggers)
        (if (Utilities|DoesObjectImplementInterface _array_element "/Game/Blueprints/Interfaces/I_FoliageEvent.I_FoliageEvent_C")
          (Class|IFoliageEvent|TriggerEvent(Message) _array_element))))))

(fn ConstructionScript
  (Components|Timeline|SetPlayRate (Variables|Default|GetGrowLeaves) (/ 1.0 (Variables|Default|GetLeavesGrowTime))))