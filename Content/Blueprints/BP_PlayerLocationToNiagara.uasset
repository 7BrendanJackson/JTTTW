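; Actor that drives the User.PlayerLocation parameter of a referenced particle actor's Niagara system.
; The construction script caches the Niagara component and seeds the parameter with the particle actor's location, which BeginPlay overrides with this actor's own.
; Once TriggerEvent enables following, Tick uses a Delay to update it about twice a second to the Character's location plus a random horizontal offset.
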(event EventTriggerEvent
  (Utilities|IsValid (Variables|Default|GetNiagaraComponent)
    (:Is%20Valid
      (Variables|Default|SetFollowPlayer true))))

(event EventTick
  (params (DeltaSeconds :type Float%20%28single-precision%29))
  (bind _returnvalue (Math|Random|RandomUnitVector))
  (bind _returnvalue_2 (Math|Vector|MakeVector (.x _returnvalue) (.y _returnvalue) 0.0))
  (bind _returnvalue_3 (Math|Vector|Normalize _returnvalue_2))
  (if (Variables|Default|GetFollowPlayer)
    (Utilities|FlowControl|Delay 0.5)
    (Niagara|SetNiagaraVariable(Vector3) (Variables|Default|GetNiagaraComponent) "User.PlayerLocation" (+ (Transformation|GetActorLocation (Variables|Default|GetCharacter)) (Math|Vector|MakeVector (* (.x _returnvalue_3) 1e+02) (* (.y _returnvalue_3) 1e+02) 0.0)))))

(event EventBeginPlay
  (bind _niagaracomponent (Variables|Default|GetNiagaraComponent))
  (Utilities|IsValid _niagaracomponent
    (:Is%20Valid
      (Niagara|SetNiagaraVariable(Vector3) _niagaracomponent "User.PlayerLocation" (Transformation|GetActorLocation)))))

(fn ConstructionScript
  (bind _output_get (Variables|Default|SetNiagaraComponent (Actor|GetComponentbyClass (Variables|Default|GetParticleSystem) "/Script/Niagara.NiagaraComponent")))
  (Niagara|SetNiagaraVariable(Vector3) _output_get "User.PlayerLocation" (Transformation|GetActorLocation (Variables|Default|GetParticleSystem))))