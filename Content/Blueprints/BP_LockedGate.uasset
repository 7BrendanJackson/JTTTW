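; BP_LockedGate is a gate that stays locked until enough medallions have been collected.
; AddMedalion increments the collected count and prints the running total.
; On Interact, a still-locked gate compares that count to the needed amount and, if it is met, unlocks permanently and prints a message.
; A timeline then swings the gate open by driving the Hinge's relative yaw.
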(event EventBeginPlay)

(event Collision|EventActorBeginOverlap
  (params (OtherActor :type Actor%20Object%20Reference)))

(event EventTick
  (params (DeltaSeconds :type Float%20%28single-precision%29)))

(event EventInteract
  (if (not (Variables|Default|GetUnlocked?))
    (if (>= (Variables|Default|GetCollectedMedalions) (Variables|Default|GetNeededMedalions))
      (Variables|Default|SetUnlocked? true)
      (Development|PrintString "GateUnlocked")
      (bind _opendoor (Timeline|Timeline PlayFromStart)
        (:Update
          (Transformation|SetRelativeRotation (Variables|Default|GetHinge) (Math|Rotator|MakeRotator 0.0 0.0 _opendoor) false false))))))

(fn ConstructionScript)

(fn AddMedalion
  (Math|Integer|IncrementInt (Variables|Default|GetCollectedMedalions)
    (:%20%20
      (Development|PrintString (Utilities|String|Append "You have " (Utilities|String|ToString(Integer) (Variables|Default|GetCollectedMedalions)) " Medalions!")))))