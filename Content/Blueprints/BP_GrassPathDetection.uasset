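; BP_GrassPathDetection tracks completion of a grass path by checking vertex paint at registered waypoints.
; CheckProgress walks waypoints in reverse, tracing down from each and querying the hit mesh's closest vertex through the runtime vertex paint and detection component, passing the array index along.
; The callback counts and removes waypoints with enough green.
; Once all succeed, Finish messages foliage-event interface triggers and activates particle triggers.
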(event GetClosestVertexDataDelegate(BPC_RuntimeVertexPaintAndDetectionComponent)
  (params (taskResultInfo :type Vertex%20Detect%20Task%20Result%20Info%20Structure) (meshVertexData :type Vertex%20Detect%20Mesh%20Data%20Struct%20Structure) (detectedMeshWithSettings :type Vertex%20Detect%20Info%20Struct%20Structure) (closestVertexInfo :type Vertex%20Detect%20Closest%20Vertex%20Data%20Result%20Struct%20Structure) (estimatedColorAtHitLocationInfo :type Vertex%20Detect%20Estimated%20Color%20at%20Hit%20Location%20Result%20Struct%20Structure) (avarageColorInAreaInfo :type Vertex%20Detect%20Avarage%20Color%20in%20Area%20Info%20Structure) (amountOfPaintedColorsOfEachChannel :type Vertex%20Detect%20Amount%20Of%20Painted%20Colors%20Of%20Each%20Channel%20Structure) (vertexColorsOnEachBone :type Vertex%20Detect%20Vertex%20Colors%20on%20Each%20Bone%20Structure) (additionalData :type Vertex%20Detect%20Additional%20Data%20to%20Pass%20Through%20Structure))
  (bind _success (Variables|Default|GetSuccess))
  (if (> (.g (.closestvertexcolors (.closestvertexgeneralinfo closestVertexInfo))) 0.2)
    (Math|Integer|IncrementInt _success
      (:%20%20
        (Utilities|Array|RemoveIndex (Variables|Default|GetWaypoints) (.passthrough_int1 additionalData))
        (if (>= _success (Variables|Default|GetNeeded))
          (CallFunction|Finish))))))

(fn ConstructionScript)

(fn CheckProgress
  (bind (_arrayindex _arrayelement) (Utilities|Array|ReverseforEachLoop (Variables|Default|GetWaypoints))
    (:LoopBody
      (bind _outhit (Collision|LineTraceByChannel (.location (Transformation|GetActorTransform _arrayelement)) (+ (.location (Transformation|GetActorTransform _arrayelement)) (* (Math|Vector|VectorDown) 5e+03)) "TraceTypeQuery3" true 0 "None"))
      (|GetClosestVertexDataonMeshNode (Variables|Default|GetBPC_RuntimeVertexPaintAndDetectionComponent) (.hitcomponent _outhit) (Utilities|Struct|MakeVertexDetectInfoStruct "(areaRangeToGetAvarageColorFrom=0.000000,VertexNormalToHitNormal_MinimumDotProductToBeAccountedFor=-1.000000)" (Utilities|Struct|MakeVertexDetectAndPaintFundementalsStruct (.location _outhit) (.normal _outhit)) "(getEstimatedColorAtHitLocation=False,onlyGetIfMeshHasMaxAmountOfVertices=True,maxAmountOfVertices=20000)" "(runCallbackDelegate=True,runCallbackInterfaces=True,includeVertexDataOnlyForLOD0=True,includeColorsOfEachBone=False,includeAmountOfPaintedColorsOfEachChannel=(includeAmountOfPaintedColorsOfEachChannel=False,includeAmountOfPaintedColorsOfEachChannel_IfMinColorAmount=0.010000),includeVertexColorData=False,includeSerializedVertexColorData=False,includeVertexPositionData=False,includeVertexNormalData=False)" "(useMultithreadingForCalculations=True,multithreadPriority=TPri_Highest)") (Utilities|Struct|MakeVertexDetectAdditionalDataToPassThrough 0 0 false false 0 0 0.0 0.0 _arrayindex 0 "0.000000,0.000000,0.000000" "0.000000,0.000000,0.000000" "0.000000,0.000000,0.000000" "0.000000,0.000000,0.000000" "0.000000,0.000000,0.000000" "0.000000,0.000000,0.000000" "0.000000,0.000000,0.000000|0.000000,0.000000,-0.000000|1.000000,1.000000,1.000000" "" "" "None" "SurfaceType_Default" "SurfaceType_Default" 0 "ECC_WorldStatic" "ObjectTypeQuery1" "(meshSource=None,meshComp=None,meshDataPerLOD=)" "(closestVertexDataSuccessfullyAcquired=False,closestVertexGeneralInfo=(closestVertexIndex=-1,closestSection=-1,closestVertexColors=(R=0.000000,G=0.000000,B=0.000000,A=0.000000),closestVertexPositionInfo=(closestVertexPositionWorld=(X=0.000000,Y=0.000000,Z=0.000000),closestVertexPositionActorLocal=(X=0.000000,Y=0.000000,Z=0.000000)),closestVertexNormalInfo=(closestVertexNormal=(X=0.000000,Y=0.000000,Z=0.000000),closestVertexNormalLocal=(X=0.000000,Y=0.000000,Z=0.000000)),closestVertexMaterial=None,closestVertexUVAtEachUVChannel=),closestVertexPhysicalSurfaceInfo=(physicsSurfaceSuccessfullyAcquired=False,mostDominantPhysicsSurfaceInfo=(mostDominantPhysicsSurface=SurfaceType_Default,mostDominantPhysicsSurfaceAsString=\"Default\",mostDominantPhysicstSurfaceValue=0.000000,mostDominantPhysicsSurfaceAtVertexColorChannels=),physicsSurface_AtDefault=(materialRegisteredToIncludeDefaultChannel=False,physicalSurfaceAtDefault=SurfaceType_Default,physicalSurfaceAsStringAtDefault=\"Default\",physicalSurfaceValueAtDefault=0.000000),physicsSurface_AtRed=(physicalSurfaceAtRedChannel=SurfaceType_Default,physicalSurfaceAsStringAtRedChannel=\"None\",physicalSurfaceValueAtRedChannel=0.000000),physicsSurface_AtGreen=(physicalSurfaceAtGreenChannel=SurfaceType_Default,physicalSurfaceAsStringAtGreenChannel=\"None\",physicalSurfaceValueAtGreenChannel=0.000000),physicsSurface_AtBlue=(physicalSurfaceAtBlueChannel=SurfaceType_Default,physicalSurfaceAsStringAtBlueChannel=\"None\",physicalSurfaceValueAtBlueChannel=0.000000),physicsSurface_AtAlpha=(physicalSurfaceAtAlphaChannel=SurfaceType_Default,physicalSurfaceAsStringAtAlphaChannel=\"None\",physicalSurfaceValueAtAlphaChannel=0.000000),physicalSurfacesAsArray=,surfacesAsStringArray=,surfaceValuesArray=))" "(estimatedColorAtHitLocationDataSuccessfullyAcquired=False,estimatedColorAtHitLocation=(R=0.000000,G=0.000000,B=0.000000,A=0.000000),physicalSurfaceInfo=(physicsSurfaceSuccessfullyAcquired=False,mostDominantPhysicsSurfaceInfo=(mostDominantPhysicsSurface=SurfaceType_Default,mostDominantPhysicsSurfaceAsString=\"Default\",mostDominantPhysicstSurfaceValue=0.000000,mostDominantPhysicsSurfaceAtVertexColorChannels=),physicsSurface_AtDefault=(materialRegisteredToIncludeDefaultChannel=False,physicalSurfaceAtDefault=SurfaceType_Default,physicalSurfaceAsStringAtDefault=\"Default\",physicalSurfaceValueAtDefault=0.000000),physicsSurface_AtRed=(physicalSurfaceAtRedChannel=SurfaceType_Default,physicalSurfaceAsStringAtRedChannel=\"None\",physicalSurfaceValueAtRedChannel=0.000000),physicsSurface_AtGreen=(physicalSurfaceAtGreenChannel=SurfaceType_Default,physicalSurfaceAsStringAtGreenChannel=\"None\",physicalSurfaceValueAtGreenChannel=0.000000),physicsSurface_AtBlue=(physicalSurfaceAtBlueChannel=SurfaceType_Default,physicalSurfaceAsStringAtBlueChannel=\"None\",physicalSurfaceValueAtBlueChannel=0.000000),physicsSurface_AtAlpha=(physicalSurfaceAtAlphaChannel=SurfaceType_Default,physicalSurfaceAsStringAtAlphaChannel=\"None\",physicalSurfaceValueAtAlphaChannel=0.000000),physicalSurfacesAsArray=,surfacesAsStringArray=,surfaceValuesArray=),worldSpaceLocationWeEstimatedTheColorAt=(X=0.000000,Y=0.000000,Z=0.000000))" "(avarageVertexColorsWithinAreaOfEffect=(R=0.000000,G=0.000000,B=0.000000,A=0.000000),avaragePhysicalSurfaceInfoBasedOffTheClosestVertexMaterial=(physicsSurfaceSuccessfullyAcquired=False,mostDominantPhysicsSurfaceInfo=(mostDominantPhysicsSurface=SurfaceType_Default,mostDominantPhysicsSurfaceAsString=\"Default\",mostDominantPhysicstSurfaceValue=0.000000,mostDominantPhysicsSurfaceAtVertexColorChannels=),physicsSurface_AtDefault=(materialRegisteredToIncludeDefaultChannel=False,physicalSurfaceAtDefault=SurfaceType_Default,physicalSurfaceAsStringAtDefault=\"Default\",physicalSurfaceValueAtDefault=0.000000),physicsSurface_AtRed=(physicalSurfaceAtRedChannel=SurfaceType_Default,physicalSurfaceAsStringAtRedChannel=\"None\",physicalSurfaceValueAtRedChannel=0.000000),physicsSurface_AtGreen=(physicalSurfaceAtGreenChannel=SurfaceType_Default,physicalSurfaceAsStringAtGreenChannel=\"None\",physicalSurfaceValueAtGreenChannel=0.000000),physicsSurface_AtBlue=(physicalSurfaceAtBlueChannel=SurfaceType_Default,physicalSurfaceAsStringAtBlueChannel=\"None\",physicalSurfaceValueAtBlueChannel=0.000000),physicsSurface_AtAlpha=(physicalSurfaceAtAlphaChannel=SurfaceType_Default,physicalSurfaceAsStringAtAlphaChannel=\"None\",physicalSurfaceValueAtAlphaChannel=0.000000),physicalSurfacesAsArray=,surfacesAsStringArray=,surfaceValuesArray=))" "(successfullyGotVerticesOfEachChannelAtTheMinAmount=False,amountOfVerticesWithAnyRedPaintedAtTheMinAmount=0.000000,amountOfRedChannelPercentPaintedAtTheMinAmount=0.000000,averageAmountOfRedColorAtTheMinAmount=0.000000,amountOfVerticesWithAnyGreenPaintedAtTheMinAmount=0.000000,amountOfGreenChannelPercentPaintedAtTheMinAmount=0.000000,averageAmountOfGreenColorAtTheMinAmount=0.000000,amountOfVerticesWithAnyBluePaintedAtTheMinAmount=0.000000,amountOfBlueChannelPercentPaintedAtTheMinAmount=0.000000,averageAmountOfBlueColorAtTheMinAmount=0.000000,amountOfVerticesWithAnyAlphaPaintedAtTheMinAmount=0.000000,amountOfAlphaChannelPercentPaintedAtTheMinAmount=0.000000,averageAmountOfAlphaColorAtTheMinAmount=0.000000)" "(successFullyGotColorsForEachBone=False,nameAndColorOfEachBone=())" "(taskSuccessfull=False,taskDuration=0.000000,anyVertexColorGotChangedByPaintJob=False)" "(getAverageColorInAreaSettings=(areaRangeToGetAvarageColorFrom=0.000000,VertexNormalToHitNormal_MinimumDotProductToBeAccountedFor=-1.000000),hitFundementals=(hitLocation=(X=0.000000,Y=0.000000,Z=0.000000),hitLocationInComponentSpace=(X=0.000000,Y=0.000000,Z=0.000000),hitNormal=(X=0.000000,Y=0.000000,Z=0.000000),hitBone=\"\",optionalFaceIndexForStaticMeshComponents=-1,runTaskFor=\"\"),getEstimatedColorAtHitLocationSettings=(getEstimatedColorAtHitLocation=False,onlyGetIfMeshHasMaxAmountOfVertices=True,maxAmountOfVertices=20000),actor=None,meshComponent=None,callbackSettings=(runCallbackDelegate=True,runCallbackInterfaces=True,includeVertexDataOnlyForLOD0=True,includeColorsOfEachBone=False,includeAmountOfPaintedColorsOfEachChannel=(includeAmountOfPaintedColorsOfEachChannel=False,includeAmountOfPaintedColorsOfEachChannel_IfMinColorAmount=0.010000),includeVertexColorData=False,includeSerializedVertexColorData=False,includeVertexPositionData=False,includeVertexNormalData=False),multiThreadSettings=(useMultithreadingForCalculations=True,multithreadPriority=TPri_Highest))" "(actor=None,meshComponent=None,callbackSettings=(runCallbackDelegate=True,runCallbackInterfaces=True,includeVertexDataOnlyForLOD0=True,includeColorsOfEachBone=False,includeAmountOfPaintedColorsOfEachChannel=(includeAmountOfPaintedColorsOfEachChannel=False,includeAmountOfPaintedColorsOfEachChannel_IfMinColorAmount=0.010000),includeVertexColorData=False,includeSerializedVertexColorData=False,includeVertexPositionData=False,includeVertexNormalData=False),multiThreadSettings=(useMultithreadingForCalculations=True,multithreadPriority=TPri_Highest))" "(hitFundementals=(hitLocation=(X=0.000000,Y=0.000000,Z=0.000000),hitLocationInComponentSpace=(X=0.000000,Y=0.000000,Z=0.000000),hitNormal=(X=0.000000,Y=0.000000,Z=0.000000),hitBone=\"\",optionalFaceIndexForStaticMeshComponents=-1,runTaskFor=\"\"),paintAtAreaSettings=(areaOfEffect=100.000000,areaOfEffectWithFullColor=10.000000,fallOffStrength=1.000000,VertexNormalToHitNormal_MinimumDotProductToGetPainted_StaticMesh=-1.000000,VertexNormalToHitNormal_MinimumDotProductToGetPainted_SkeletalMesh=-1.000000),getEstimatedColorAtHitLocationSettings=(getEstimatedColorAtHitLocation=False,onlyGetIfMeshHasMaxAmountOfVertices=True,maxAmountOfVertices=20000),detection=(runGetClosestVertexDataOnMeshBeforeApplyingPaint=False,runGetClosestVertexDataOnMeshAfterApplyingPaint=False,getAverageColorInAreaSettings=(areaRangeToGetAvarageColorFrom=0.000000,VertexNormalToHitNormal_MinimumDotProductToBeAccountedFor=-1.000000),useCustomHitFundementalsForDetection=False,detectHitFundementals=(hitLocation=(X=0.000000,Y=0.000000,Z=0.000000),hitLocationInComponentSpace=(X=0.000000,Y=0.000000,Z=0.000000),hitNormal=(X=0.000000,Y=0.000000,Z=0.000000),hitBone=\"\",optionalFaceIndexForStaticMeshComponents=-1,runTaskFor=\"\")),applyVertexColorSettings=(applyVertexColorSetting=EAddVertexColor,redColor=0.000000,redColorCondition=(ifVertexColorIsWithinRange=,ifVertexHasLineOfSightTo=,ifVertexIsOnBone=,applyColorStrengthIfConditionIsNotMet=False,colorStrengthIfConditionIsNotMet=0.000000),greenColor=0.000000,greenColorCondition=(ifVertexColorIsWithinRange=,ifVertexHasLineOfSightTo=,ifVertexIsOnBone=,applyColorStrengthIfConditionIsNotMet=False,colorStrengthIfConditionIsNotMet=0.000000),blueColor=0.000000,blueColorCondition=(ifVertexColorIsWithinRange=,ifVertexHasLineOfSightTo=,ifVertexIsOnBone=,applyColorStrengthIfConditionIsNotMet=False,colorStrengthIfConditionIsNotMet=0.000000),alphaColor=0.000000,alphaColorCondition=(ifVertexColorIsWithinRange=,ifVertexHasLineOfSightTo=,ifVertexIsOnBone=,applyColorStrengthIfConditionIsNotMet=False,colorStrengthIfConditionIsNotMet=0.000000)),limitPaintColor=(usePaintLimits=False,limitColorIfTheColorWasAlreadyOverTheLimit=False,paintLimitOnRedChannel=1.000000,paintLimitOnGreenChannel=1.000000,paintLimitOnBlueChannel=1.000000,paintLimitOnAlphaChannel=1.000000),limitPaintToSpecifiedNormal=(limitPaintingToSpecifiedWorldNormal=False,worldNormal=(X=0.000000,Y=0.000000,Z=0.000000),errorTolerance=0.100000),overrideLOD=(overrideLODToPaintUpTo=False,amountOfLODsToPaint=1),affectClothPhysics=True,actor=None,meshComponent=None,callbackSettings=(runCallbackDelegate=True,runCallbackInterfaces=True,includeVertexDataOnlyForLOD0=True,includeColorsOfEachBone=False,includeAmountOfPaintedColorsOfEachChannel=(includeAmountOfPaintedColorsOfEachChannel=False,includeAmountOfPaintedColorsOfEachChannel_IfMinColorAmount=0.010000),includeVertexColorData=False,includeSerializedVertexColorData=False,includeVertexPositionData=False,includeVertexNormalData=False),multiThreadSettings=(useMultithreadingForCalculations=True,multithreadPriority=TPri_Highest))" "(componentsToCheckIfIsWithin=,extraExtentToApplyPaintOn=0.000000,areaOfEffectWithFullColor=0.000000,fallOffStrength=0.000000,falloffType=FromComponentCenter,applyVertexColorSettings=(applyVertexColorSetting=EAddVertexColor,redColor=0.000000,redColorCondition=(ifVertexColorIsWithinRange=,ifVertexHasLineOfSightTo=,ifVertexIsOnBone=,applyColorStrengthIfConditionIsNotMet=False,colorStrengthIfConditionIsNotMet=0.000000),greenColor=0.000000,greenColorCondition=(ifVertexColorIsWithinRange=,ifVertexHasLineOfSightTo=,ifVertexIsOnBone=,applyColorStrengthIfConditionIsNotMet=False,colorStrengthIfConditionIsNotMet=0.000000),blueColor=0.000000,blueColorCondition=(ifVertexColorIsWithinRange=,ifVertexHasLineOfSightTo=,ifVertexIsOnBone=,applyColorStrengthIfConditionIsNotMet=False,colorStrengthIfConditionIsNotMet=0.000000),alphaColor=0.000000,alphaColorCondition=(ifVertexColorIsWithinRange=,ifVertexHasLineOfSightTo=,ifVertexIsOnBone=,applyColorStrengthIfConditionIsNotMet=False,colorStrengthIfConditionIsNotMet=0.000000)),limitPaintColor=(usePaintLimits=False,limitColorIfTheColorWasAlreadyOverTheLimit=False,paintLimitOnRedChannel=1.000000,paintLimitOnGreenChannel=1.000000,paintLimitOnBlueChannel=1.000000,paintLimitOnAlphaChannel=1.000000),limitPaintToSpecifiedNormal=(limitPaintingToSpecifiedWorldNormal=False,worldNormal=(X=0.000000,Y=0.000000,Z=0.000000),errorTolerance=0.100000),overrideLOD=(overrideLODToPaintUpTo=False,amountOfLODsToPaint=1),affectClothPhysics=True,actor=None,meshComponent=None,callbackSettings=(runCallbackDelegate=True,runCallbackInterfaces=True,includeVertexDataOnlyForLOD0=True,includeColorsOfEachBone=False,includeAmountOfPaintedColorsOfEachChannel=(includeAmountOfPaintedColorsOfEachChannel=False,includeAmountOfPaintedColorsOfEachChannel_IfMinColorAmount=0.010000),includeVertexColorData=False,includeSerializedVertexColorData=False,includeVertexPositionData=False,includeVertexNormalData=False),multiThreadSettings=(useMultithreadingForCalculations=True,multithreadPriority=TPri_Highest))" "(paintOnRandomVerticesSettings=(paintAtRandomVerticesSpreadOutOverTheEntireMesh=False,paintAtRandomVerticesSpreadOutOverTheEntireMesh_PercentToPaint=10.000000,paintAtRandomVerticesSpreadOutOverTheEntireMesh_PropogateLOD0ToAllLODsMethod=ModifiedEngineMethod),applyVertexColorSettings=(applyVertexColorSetting=EAddVertexColor,redColor=0.000000,redColorCondition=(ifVertexColorIsWithinRange=,ifVertexHasLineOfSightTo=,ifVertexIsOnBone=,applyColorStrengthIfConditionIsNotMet=False,colorStrengthIfConditionIsNotMet=0.000000),greenColor=0.000000,greenColorCondition=(ifVertexColorIsWithinRange=,ifVertexHasLineOfSightTo=,ifVertexIsOnBone=,applyColorStrengthIfConditionIsNotMet=False,colorStrengthIfConditionIsNotMet=0.000000),blueColor=0.000000,blueColorCondition=(ifVertexColorIsWithinRange=,ifVertexHasLineOfSightTo=,ifVertexIsOnBone=,applyColorStrengthIfConditionIsNotMet=False,colorStrengthIfConditionIsNotMet=0.000000),alphaColor=0.000000,alphaColorCondition=(ifVertexColorIsWithinRange=,ifVertexHasLineOfSightTo=,ifVertexIsOnBone=,applyColorStrengthIfConditionIsNotMet=False,colorStrengthIfConditionIsNotMet=0.000000)),limitPaintColor=(usePaintLimits=False,limitColorIfTheColorWasAlreadyOverTheLimit=False,paintLimitOnRedChannel=1.000000,paintLimitOnGreenChannel=1.000000,paintLimitOnBlueChannel=1.000000,paintLimitOnAlphaChannel=1.000000),limitPaintToSpecifiedNormal=(limitPaintingToSpecifiedWorldNormal=False,worldNormal=(X=0.000000,Y=0.000000,Z=0.000000),errorTolerance=0.100000),overrideLOD=(overrideLODToPaintUpTo=False,amountOfLODsToPaint=1),affectClothPhysics=True,actor=None,meshComponent=None,callbackSettings=(runCallbackDelegate=True,runCallbackInterfaces=True,includeVertexDataOnlyForLOD0=True,includeColorsOfEachBone=False,includeAmountOfPaintedColorsOfEachChannel=(includeAmountOfPaintedColorsOfEachChannel=False,includeAmountOfPaintedColorsOfEachChannel_IfMinColorAmount=0.010000),includeVertexColorData=False,includeSerializedVertexColorData=False,includeVertexPositionData=False,includeVertexNormalData=False),multiThreadSettings=(useMultithreadingForCalculations=True,multithreadPriority=TPri_Highest))" "(colorSnippetTag=(TagName=\"\"),randomizeAnyColorSnippetTagUnderThisCategory=(TagName=\"\"),colorSnippetID=\"\",colorSnippetDataAssetSnippetIsStoredIn=None,overrideLOD=(overrideLODToPaintUpTo=False,amountOfLODsToPaint=1),affectClothPhysics=True,actor=None,meshComponent=None,callbackSettings=(runCallbackDelegate=True,runCallbackInterfaces=True,includeVertexDataOnlyForLOD0=True,includeColorsOfEachBone=False,includeAmountOfPaintedColorsOfEachChannel=(includeAmountOfPaintedColorsOfEachChannel=False,includeAmountOfPaintedColorsOfEachChannel_IfMinColorAmount=0.010000),includeVertexColorData=False,includeSerializedVertexColorData=False,includeVertexPositionData=False,includeVertexNormalData=False),multiThreadSettings=(useMultithreadingForCalculations=True,multithreadPriority=TPri_Highest))" "(overrideLOD=(overrideLODToPaintUpTo=False,amountOfLODsToPaint=1),affectClothPhysics=True,actor=None,meshComponent=None,callbackSettings=(runCallbackDelegate=True,runCallbackInterfaces=True,includeVertexDataOnlyForLOD0=True,includeColorsOfEachBone=False,includeAmountOfPaintedColorsOfEachChannel=(includeAmountOfPaintedColorsOfEachChannel=False,includeAmountOfPaintedColorsOfEachChannel_IfMinColorAmount=0.010000),includeVertexColorData=False,includeSerializedVertexColorData=False,includeVertexPositionData=False,includeVertexNormalData=False),multiThreadSettings=(useMultithreadingForCalculations=True,multithreadPriority=TPri_Highest))")))))

(fn RegisterWaypoint
  (params (New%20Waypoint :type BP%20Grass%20Detection%20Waypoint%20Object%20Reference))
  (bind _returnvalue (Utilities|Array|Add (Variables|Default|GetWaypoints) New%20Waypoint))
  (Variables|Default|SetNeeded (+ _returnvalue 1)))

(fn Finish
  (for _array_element (Variables|Default|GetFinishTriggers)
    (if (Utilities|DoesObjectImplementInterface _array_element "/Game/Blueprints/Interfaces/I_FoliageEvent.I_FoliageEvent_C")
      (Class|IFoliageEvent|TriggerEvent(Message) _array_element)))
  (for _array_element_2 (Variables|Default|GetParticleTriggers)
    (Components|Activation|Activate _array_element_2 false)))