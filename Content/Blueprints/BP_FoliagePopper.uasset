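; BP_FoliagePopper is an actor that paints green vertex color onto the mesh beneath it for a timed burst.
; TriggerEvent or the 2 key starts Fire, which raises the Firing flag for FireTime.
; While Firing, Tick traces straight down and uses the Runtime Vertex Paint and Detection component to paint at the hit.
; Spread, FullForceDistance and Falloff shape the area, while Force scaled by DeltaSeconds sets the strength.
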(event Custom|Fire
  (Variables|Default|SetFiring true)
  (Utilities|FlowControl|Delay (Variables|Default|GetFireTime))
  (Variables|Default|SetFiring false))

(event EventTriggerEvent
  (CallFunction|Fire))

(event EventTick
  (params (DeltaSeconds :type Float%20%28single-precision%29))
  (bind _returnvalue (Transformation|GetActorLocation))
  (if (Variables|Default|GetFiring)
    (bind (_outhit _returnvalue_2) (Collision|LineTraceByChannel _returnvalue (+ _returnvalue (* (Math|Vector|VectorDown) 5e+03)) "TraceTypeQuery3" true 0 "None"))
    (if _returnvalue_2
      (|PaintatLocationNode (Variables|Default|GetBPC_RuntimeVertexPaintAndDetectionComponent) (.hitcomponent _outhit) (Utilities|Struct|MakeVertexPaintAtLocationStruct (Utilities|Struct|MakeVertexDetectAndPaintFundementalsStruct (.location _outhit) (.normal _outhit) (.bonename _outhit) (.faceindex _outhit)) (Utilities|Struct|MakeVertexDetectPaintAtLocationAreaSettings (Variables|Default|GetSpread) (Variables|Default|GetFullForceDistance) (Variables|Default|GetFalloff)) "(getEstimatedColorAtHitLocation=False,onlyGetIfMeshHasMaxAmountOfVertices=True,maxAmountOfVertices=20000)" "(runGetClosestVertexDataOnMeshBeforeApplyingPaint=False,runGetClosestVertexDataOnMeshAfterApplyingPaint=False,getAverageColorInAreaSettings=(areaRangeToGetAvarageColorFrom=0.000000,VertexNormalToHitNormal_MinimumDotProductToBeAccountedFor=-1.000000),useCustomHitFundementalsForDetection=False,detectHitFundementals=(hitLocation=(X=0.000000,Y=0.000000,Z=0.000000),hitLocationInComponentSpace=(X=0.000000,Y=0.000000,Z=0.000000),hitNormal=(X=0.000000,Y=0.000000,Z=0.000000),hitBone=\"\",optionalFaceIndexForStaticMeshComponents=-1,runTaskFor=\"\"))" (Utilities|Struct|MakeVertexDetectRGBAStruct "EAddVertexColor" 0.0 "(ifVertexColorIsWithinRange=,ifVertexHasLineOfSightTo=,ifVertexIsOnBone=,applyColorStrengthIfConditionIsNotMet=False,colorStrengthIfConditionIsNotMet=0.000000)" (* DeltaSeconds (Variables|Default|GetForce)) (Utilities|Struct|MakeVertexDetectPaintColorConditionStruct 0 0 0 false 0.1)) "(usePaintLimits=False,limitColorIfTheColorWasAlreadyOverTheLimit=False,paintLimitOnRedChannel=1.000000,paintLimitOnGreenChannel=1.000000,paintLimitOnBlueChannel=1.000000,paintLimitOnAlphaChannel=1.000000)" "(limitPaintingToSpecifiedWorldNormal=False,worldNormal=(X=0.000000,Y=0.000000,Z=0.000000),errorTolerance=0.100000)" "(overrideLODToPaintUpTo=False,amountOfLODsToPaint=1)" true "(runCallbackDelegate=True,runCallbackInterfaces=True,includeVertexDataOnlyForLOD0=True,includeColorsOfEachBone=False,includeAmountOfPaintedColorsOfEachChannel=(includeAmountOfPaintedColorsOfEachChannel=False,includeAmountOfPaintedColorsOfEachChannel_IfMinColorAmount=0.010000),includeVertexColorData=False,includeSerializedVertexColorData=False,includeVertexPositionData=False,includeVertexNormalData=False)" "(useMultithreadingForCalculations=True,multithreadPriority=TPri_Highest)")))))

(event Input|KeyboardEvents|2
  (params (Key :type Key%20Structure))
  (:Pressed
    (CallFunction|Fire)))

(fn ConstructionScript)