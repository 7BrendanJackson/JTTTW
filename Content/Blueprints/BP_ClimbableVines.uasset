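; Climbable vine actor that grows once on a trigger event (or the 1 key) and then acts as a ladder for the Regrowth character.
; A timeline scaled by VineGrowTime feeds growth into the vine material through custom primitive data and marks the vines climbable when grown.
; Box overlap below Highpoint enables the character's ladder state along the arrow's reversed forward vector.
; Leaving clears that state, adding a forward-and-up boost if above Highpoint.
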(event OnComponentBeginOverlap(Box)
  (params (OverlappedComponent :type Primitive%20Component%20Object%20Reference) (OtherActor :type Actor%20Object%20Reference) (OtherComp :type Primitive%20Component%20Object%20Reference) (OtherBodyIndex :type Integer) (bFromSweep :type Boolean) (SweepResult :type Hit%20Result%20Structure%20%28by%20ref%29))
  (bind _asbp_regrowth_character (Utilities|Casting|CastToBP_RegrowthCharacter OtherActor))
  (if (Variables|Default|GetVinesGrown)
    (if (> (.z (Transformation|GetWorldLocation (Variables|Default|GetHighpoint))) (.z (Transformation|GetActorLocation _asbp_regrowth_character)))
      (Default|ChangeLadderState _asbp_regrowth_character true (* (Math|Vector|GetForwardVector (Variables|Default|GetArrow)) -1.0)))))

(event OnComponentEndOverlap(Box)
  (params (OverlappedComponent :type Primitive%20Component%20Object%20Reference) (OtherActor :type Actor%20Object%20Reference) (OtherComp :type Primitive%20Component%20Object%20Reference) (OtherBodyIndex :type Integer))
  (bind _asbp_regrowth_character (Utilities|Casting|CastToBP_RegrowthCharacter OtherActor))
  (if (Variables|/Game/ThirdPerson/Blueprints/BP_RegrowthCharacter.BP_RegrowthCharacter_C|GetOnLadder? _asbp_regrowth_character)
    (if (> (.z (Transformation|GetActorLocation _asbp_regrowth_character)) (.z (Transformation|GetWorldLocation (Variables|Default|GetHighpoint))))
      (Physics|AddImpulse (Variables|/Script/Engine.Character|GetCharacterMovement _asbp_regrowth_character) (+ (* (Transformation|GetActorForwardVector _asbp_regrowth_character) 2.5e+02) "0.000000,0.000000,250.000000") true))
    (Default|ChangeLadderState _asbp_regrowth_character false "0, 0, 0")))

(event Custom|GrowVines
  (bind _growing (Timeline|VinesGrowing Play)
    (:Update
      (Rendering|Material|SetCustomPrimitiveDataFloat (Variables|Default|GetVines) 0 _growing))
    (:MarkAsGrown
      (Variables|Default|SetVinesGrown true))))

(event EventTriggerEvent
  (Utilities|FlowControl|DoOnce false
    (:Completed
      (CallFunction|GrowVines))))

(event Input|KeyboardEvents|1
  (params (Key :type Key%20Structure))
  (:Pressed
    (Utilities|FlowControl|DoOnce false
      (:Completed
        (CallFunction|GrowVines)))))

(fn ConstructionScript
  (Components|Timeline|SetPlayRate (Variables|Default|GetVinesGrowing) (/ 1.0 (Variables|Default|GetVineGrowTime))))